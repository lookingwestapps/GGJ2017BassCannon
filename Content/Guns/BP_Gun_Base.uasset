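; BP_Gun_Base is a base gun that fires projectiles meant to hit vases of a specific color.
; ShootFunc spawns a short-lived BP_Projectile past the muzzle with the gun's amplitude, frequency, material and an attached shot sound.
; The gun mesh's collision object type becomes a blocking channel on the projectile, selecting which vase color it hits.
; Each shot also plays video on the ring's media player while the Fadeout timeline animates the ring's opacity.
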(event EventBeginPlay)

(event Collision|EventActorBeginOverlap
  (params (OtherActor :type Actor%20Object%20Reference)))

(event EventShoot
  (CallFunction|ShootFunc)
  (bind _opacity (Timeline|Fadeout PlayFromStart)
    (:Update
      (Rendering|Material|SetScalarParameterValue (Variables|Default|GetRingDynamicMaterial) "Opacity" _opacity :!class /Script/Engine.MaterialInstanceDynamic))))

(event EventTick
  (params (DeltaSeconds :type Float%20%28single-precision%29)))

(fn ConstructionScript)

(fn ShootFunc
  (bind _defaultsceneroot (Variables|Default|GetDefaultSceneRoot))
  (bind _ringmediaplayer (Variables|Default|GetRingMediaPlayer))
  ;[1 1 1] NOTE: A Shoot "Message" is sent to the EventGraph before calling this function
  ;[1 1 1] Spawn projectile at Hand
  (bind _returnvalue (Game|SpawnActorfromClass "/Game/BP_Projectile.BP_Projectile_C" (Transformation|GetWorldTransform _defaultsceneroot) "Undefined" 0 0))
  ;[1 1 1] Set which vase color this projectile should hit by turning on that collision channel
  (Collision|SetCollisionResponsetoChannel (Variables|/Game/BP_Projectile.BP_Projectile_C|GetCapsule _returnvalue) (Collision|GetCollisionObjectType (Variables|Default|GetStaticMesh)) "ECR_Block")
  (Variables|/Game/BP_Projectile.BP_Projectile_C|SetAmplitude _returnvalue (Variables|Default|GetAmplitude))
  (Variables|/Game/BP_Projectile.BP_Projectile_C|SetFrequency _returnvalue (Variables|Default|GetFrequency))
  ;[1 1 1] Set the projectile material that the gun specifies
  (Rendering|Material|SetMaterial (Variables|/Game/BP_Projectile.BP_Projectile_C|GetSphere _returnvalue) 0 (Variables|Default|GetProjectileMaterial))
  ;[1 1 1] Move projectile to front of gun muzzle
  (Transformation|AddRelativeLocation (Variables|/Game/BP_Projectile.BP_Projectile_C|GetDefaultSceneRoot _returnvalue) (Math|Vector|RotateVector (Math|Vector|MakeVector 1.5e+02 -2e+01 0.0) (Transformation|GetWorldRotation _defaultsceneroot)) false false)
  (Actor|SetLifeSpan _returnvalue 5.0) ; SET HOW LONG PROJECTILE LIVE
  ;[1 1 1] Play Shot Sound
  (Audio|SpawnSoundAttached (Variables|Default|GetShootSound) (Variables|/Game/BP_Projectile.BP_Projectile_C|GetSphere _returnvalue) "None" "0, 0, 0" "0, 0, 0" "KeepRelativeOffset" false 1.0 1.0 0.0 "/Game/Audio/ShotFalloffAttenuation.ShotFalloffAttenuation")
  ;[1 1 1] Play Video on Media Player Ring
  (Media|MediaPlayer|OpenSource _ringmediaplayer (Variables|Default|GetRingMediaSource))
  (Media|MediaPlayer|Play _ringmediaplayer :!class /Script/MediaAssets.MediaPlayer))