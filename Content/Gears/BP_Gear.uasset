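; BP_Gear is a gear actor that carries eight targets and spins continuously.
; Tick rolls the root component by RotationSpeed scaled by delta time.
; The construction script applies TargetMesh to all eight target components and GearMaterial to the cylinder.
; An unconnected loop that would space the targets evenly around the gear with sine and cosine never runs.
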(event EventBeginPlay)

(event Collision|EventActorBeginOverlap
  (params (OtherActor :type Actor%20Object%20Reference)))

(event EventTick
  (params (DeltaSeconds :type Float%20%28single-precision%29))
  ;[1 1 1] Rotate Platform
  (Transformation|AddLocalRotation (Variables|Default|GetDefaultSceneRoot) (Math|Rotator|MakeRotator (* DeltaSeconds (Variables|Default|GetRotationSpeed)) 0.0 0.0) false false))

(fn ConstructionScript
  (bind _output_get (Variables|Default|SetTargetArray (Utilities|Array|MakeArray (Variables|Default|GetTarget1) (Variables|Default|GetTarget2) (Variables|Default|GetTarget3) (Variables|Default|GetTarget4) (Variables|Default|GetTarget5) (Variables|Default|GetTarget6) (Variables|Default|GetTarget7) (Variables|Default|GetTarget8))))
  ;[1 1 1] Set the static mesh for the targets
  (for _array_element _output_get
    (Components|StaticMesh|SetStaticMesh _array_element (Variables|Default|GetTargetMesh)))
  ;[1 1 1] Set Gear Material
  (Rendering|Material|SetMaterial (Variables|Default|GetCylinder) 0 (Variables|Default|GetGearMaterial)))