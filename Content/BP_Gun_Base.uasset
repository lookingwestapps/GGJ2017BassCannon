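; BP_Gun_Base is a base gun Blueprint whose Shoot function fires a BP_Projectile.
; Shoot spawns the projectile at the gun's root, passes it the gun's Amplitude, Frequency and material, then nudges it to the muzzle with an offset rotated by the gun's orientation.
; It also sets a fixed projectile lifespan and plays the shot sound attached to the projectile.
; The event graph and construction script are empty.
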(event EventBeginPlay)

(event Collision|EventActorBeginOverlap
  (params (OtherActor :type Actor%20Object%20Reference)))

(event EventTick
  (params (DeltaSeconds :type Float%20%28single-precision%29)))

(fn ConstructionScript)

(fn Shoot
  (bind _defaultsceneroot (Variables|Default|GetDefaultSceneRoot))
  ;[1 1 1] Spawn projectile at Hand
  (bind _returnvalue (Game|SpawnActorfromClass "/Game/BP_Projectile.BP_Projectile_C" (Transformation|GetWorldTransform _defaultsceneroot) "Undefined" 0 0))
  (Variables|/Game/BP_Projectile.BP_Projectile_C|SetAmplitude _returnvalue (Variables|Default|GetAmplitude))
  (Variables|/Game/BP_Projectile.BP_Projectile_C|SetFrequency _returnvalue (Variables|Default|GetFrequency))
  ;[1 1 1] Set the projectile material that the gun specifies
  (Rendering|Material|SetMaterial (Variables|/Game/BP_Projectile.BP_Projectile_C|GetSphere _returnvalue) 0 (Variables|Default|GetProjectileMaterial))
  ;[1 1 1] Move projectile to front of gun muzzle
  (Transformation|AddRelativeLocation (Variables|/Game/BP_Projectile.BP_Projectile_C|GetDefaultSceneRoot _returnvalue) (Math|Vector|RotateVector (Math|Vector|MakeVector 1.5e+02 -2e+01 0.0) (Transformation|GetWorldRotation _defaultsceneroot)) false false)
  (Actor|SetLifeSpan _returnvalue 8.0) ; SET HOW LONG PROJECTILE LIVE
  ;[1 1 1] Play Shot Sound
  (Audio|SpawnSoundAttached (Variables|Default|GetShootSound) (Variables|/Game/BP_Projectile.BP_Projectile_C|GetDefaultSceneRoot _returnvalue)))