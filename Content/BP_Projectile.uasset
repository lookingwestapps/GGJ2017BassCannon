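; Projectile actor whose Sphere component pulses in size as it flies.
; Tick accumulates live time and feeds it through a sine wave, offset to stay positive and scaled by Amplitude and Frequency, to drive the sphere's Y and Z scale while X stays fixed.
; It then zeroes the sphere's relative rotation each frame.
; An unconnected branch that would oscillate the sphere's position instead is left unused.
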(event EventBeginPlay)

(event Collision|EventActorBeginOverlap
  (params (OtherActor :type Actor%20Object%20Reference)))

(event EventTick
  (params (DeltaSeconds :type Float%20%28single-precision%29))
  ;[1 1 1] Make projectile scale in sine wave pattern as it flies
  (bind _output_get (Variables|Default|SetTotalLiveTimer (+ DeltaSeconds (Variables|Default|GetTotalLiveTimer))))
  (Transformation|SetRelativeScale3D (Variables|Default|GetSphere) (Math|Vector|MakeVector 1.0 (* (+ (Math|Trig|Sin(Radians) (* _output_get (Variables|Default|GetFrequency))) 1.3) (Variables|Default|GetAmplitude)) (* (+ (Math|Trig|Sin(Radians) (* _output_get (Variables|Default|GetFrequency))) 1.3) (Variables|Default|GetAmplitude)))) ; Scale in a sine wave pattern
  (Transformation|SetRelativeRotation (Variables|Default|GetSphere) (Math|Rotator|MakeRotator 0.0 0.0 0.0) false false) ; Make sure projectile is pointing in the correct direction
)

(fn ConstructionScript)